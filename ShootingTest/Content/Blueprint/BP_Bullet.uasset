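; BP_Bullet is a projectile actor that flies straight along its forward vector and destroys enemies it overlaps.
; Tick calls a Translate helper that offsets the location by normalized direction, Speed and frame delta time, without sweeping.
; On overlap with a BP_Enemy, it spawns an explosion particle at the enemy's location, then destroys both the enemy and itself.
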(event `self.ReceiveActorBeginOverlap`
  (params (OtherActor :type "Actor Object Reference"))
  (bind _asbp_enemy (cast `/Game/Blueprint/BP_Enemy` OtherActor))
  (`GameplayStatics.SpawnEmitterAtLocation` "/Game/StarterContent/Particles/P_Explosion.P_Explosion" (`self.K2_GetActorLocation` _asbp_enemy))
  (`self.K2_DestroyActor` _asbp_enemy)
  (`self.K2_DestroyActor`))

(event `self.ReceiveTick`
  (params (DeltaSeconds :type "Float (single-precision)"))
  ;[1 1 1] 나의 전방 방향으로 이동하고 싶다.               P = P0 + VT
  (`self.Translate` (`self.GetActorForwardVector`) (`self.Speed`)))

(fn `Translate`
  (params (Direction :type "Vector Structure") (Speed :type "Float (double-precision)") (Sweep :type Boolean))
  (`self.K2_SetActorLocation` (+ (* (`KismetMathLibrary.Normal` Direction) Speed (`GameplayStatics.GetWorldDeltaSeconds`)) (`self.K2_GetActorLocation`)) Sweep))

(fn `UserConstructionScript`)