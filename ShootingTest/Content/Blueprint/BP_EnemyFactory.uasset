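; Enemy factory actor that repeatedly spawns BP_Enemy during play.
; BeginPlay starts a looping timer that calls MakeEnemy by function name every MakeTime seconds.
; MakeEnemy spawns at the Arrow component's world transform, ignoring collisions.
; Unconnected nodes hold alternative timing approaches, a delta-time accumulator and a timer by event, which never run.
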(event `Event MakeEnemy`)

(event `self.ReceiveBeginPlay`
  (`KismetSystemLibrary.K2_SetTimer` null "MakeEnemy" (`self.MakeTime`) true))

(event `self.ReceiveTick`
  (params (DeltaSeconds :type "Float (single-precision)")))

(fn `MakeEnemy`
  (`|SpawnActorFromClass` "/Game/Blueprint/BP_Enemy.BP_Enemy_C" (`SceneComponent.K2_GetComponentToWorld` (`self.Arrow`)) "AlwaysSpawn" "MultiplyWithRoot" null null))

(fn `UserConstructionScript`)