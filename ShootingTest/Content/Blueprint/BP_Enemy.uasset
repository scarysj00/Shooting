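; BP_Enemy is an enemy actor that flies in a straight line and destroys the player on contact.
; On BeginPlay it randomly locks its direction, 30% of the time toward the player's current position, otherwise along its forward vector.
; Tick moves it through a Translate helper using frame-time-scaled speed without sweep.
; Overlapping BP_Player spawns an explosion at the player and destroys both actors.
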(event `self.ReceiveBeginPlay`
  ;[1 1 1] 적이 태어날 때(BeginPlay) 방향을 30% 확률로 플레이어를 향하는 방향        (타겟 - 나)과 나머지 확률은  앞 방향으로 정하고 싶다.
  (if (< (`KismetMathLibrary.RandomIntegerInRange` 0 9) 3)
    ;[1 1 1] 플레이어를 찾아서 그 방향을 구한 후 Direction 변수에 넣어주고 싶다.
    (set `self.Direction` (`KismetMathLibrary.Normal` (- (`self.K2_GetActorLocation` (`GameplayStatics.GetPlayerPawn` 0)) (`self.K2_GetActorLocation`))))
    (else
      (set `self.Direction` (`self.GetActorForwardVector`)))))

(event `self.ReceiveTick`
  (params (DeltaSeconds :type "Float (single-precision)"))
  ;[1 1 1] 살아가면서(Tick) 계속 이 확률로 이동하고 싶다
  (`self.Translate` (`self.Direction`) (`self.Speed`)))

(event `self.ReceiveActorBeginOverlap`
  (params (OtherActor :type "Actor Object Reference"))
  (bind _asbp_player (cast `/Game/Blueprint/BP_Player` OtherActor))
  (`GameplayStatics.SpawnEmitterAtLocation` "/Game/StarterContent/Particles/P_Explosion.P_Explosion" (`self.K2_GetActorLocation` _asbp_player))
  (`self.K2_DestroyActor` _asbp_player)
  (`self.K2_DestroyActor`))

(fn `Translate`
  (params (Direction :type "Vector Structure") (Speed :type "Float (double-precision)") (Sweep :type Boolean))
  (`self.K2_SetActorLocation` (+ (* (`KismetMathLibrary.Normal` Direction) Speed (`GameplayStatics.GetWorldDeltaSeconds`)) (`self.K2_GetActorLocation`)) Sweep))

(fn `UserConstructionScript`)