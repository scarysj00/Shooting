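; Player actor for a shooter that moves on its right/up plane from input and fires bullets while Fire is held.
; Tick translates it by normalized input direction, speed and delta time, without sweeping for collision.
; Pressing Fire spawns a BP_Bullet at the Arrow component and starts a looping MakeBullet timer, which release clears.
; An unconnected auto-fire branch holds the only fire sound call, so it never plays.
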(event `self.ReceiveTick`
  (params (DeltaSeconds :type "Float (single-precision)"))
  (`|ExecutionSequence`
    (:`then_0`
      ;[1 1 1] 사용자의 입력에 따라 이동하고 싶다. P = P0 + vt (이동 위치 =  현재 위치 + 속도(방향 * 크기) * 시간 )
      (`self.Translate` (`self.GetDirection`) (`self.Speed`)))))

(event `InputAction|Fire`
  (params (Key :type "Key Structure"))
  (:`Pressed`
    (bind _returnvalue (`KismetSystemLibrary.K2_SetTimer` null "MakeBullet" (`self.FireInterval`) true))
    (set `self.MakeBulletTimerHandle` _returnvalue)
    (`self.MakeBullet`))
  (:`Released`
    (`KismetSystemLibrary.K2_ClearAndInvalidateTimerHandle` (`self.MakeBulletTimerHandle`))))

(fn `GetDirection`
  (returns (Direction :type "Vector Structure"))
  (return (`KismetMathLibrary.Normal` (+ (* (`self.GetInputAxisValue`) (`self.GetActorRightVector`)) (* (`self.GetInputAxisValue`) (`self.GetActorUpVector`))))))

(fn `MakeBullet`
  (`|SpawnActorFromClass` "/Game/Blueprint/BP_Bullet.BP_Bullet_C" (`SceneComponent.K2_GetComponentToWorld` (`self.Arrow`)) "AlwaysSpawn" "MultiplyWithRoot" null null))

(fn `Translate`
  (params (Direction :type "Vector Structure") (Speed :type "Float (double-precision)") (Sweep :type Boolean))
  (`self.K2_SetActorLocation` (+ (* (`KismetMathLibrary.Normal` Direction) Speed (`GameplayStatics.GetWorldDeltaSeconds`)) (`self.K2_GetActorLocation`)) Sweep))

(fn `UserConstructionScript`)